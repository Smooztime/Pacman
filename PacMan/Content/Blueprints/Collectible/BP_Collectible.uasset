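; BP_Collectible is a collectible actor that animates a Bag component, with no pickup logic in its graphs.
; On BeginPlay the BagMove timeline drives a lerp of the bag's relative location between StartPoint and Destination.
; Tick spins the whole actor around local yaw at BagRotation, scaled by delta time for frame-rate independence.
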(event `self.ReceiveBeginPlay`
  (bind (_direction _alpha) (`Timeline|BagMove`)
    (:`Update`
      (`SceneComponent.K2_SetRelativeLocation` (`self.Bag`) (`KismetMathLibrary.VLerp` (`self.StartPoint`) (`self.Destination`) _alpha) false false))))

(event `self.ReceiveTick`
  (params (DeltaSeconds :type "Float (single-precision)"))
  (`self.K2_AddActorLocalRotation` (`KismetMathLibrary.MakeRotator` 0.0 0.0 (* DeltaSeconds (`self.BagRotation`)))))

(fn `UserConstructionScript`)