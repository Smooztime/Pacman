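; Base character Blueprint that provides player movement through Enhanced Input.
; On possession it adds the IMC_Input mapping context to the player controller's subsystem, printing a message if no player controller is found.
; IA_Movement feeds a Movement function that maps X to world right and Y to world forward, so movement follows fixed world axes independent of camera or actor rotation.
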(event `self.ReceivePossessed`
  (params (NewController :type "Controller Object Reference"))
  (`self.SetUpInput`))

(event `EnhancedInput|/Game/Blueprints/Input/IA_Movement`
  (params (ActionValue :type "Vector2D Structure") (ElapsedSeconds :type "Float (double-precision)") (TriggeredSeconds :type "Float (double-precision)") (InputAction :type "InputAction Object Reference" :default "/Game/Blueprints/Input/IA_Movement.IA_Movement"))
  (:`Triggered`
    (`self.Movement` ActionValue)))

(fn `Movement`
  (params (AxisValue :type "Vector2D Structure"))
  (`self.AddMovementInput` (`KismetMathLibrary.Vector_Right`) AxisValue_X)
  (`self.AddMovementInput` (`KismetMathLibrary.Vector_Forward`) AxisValue_Y))

(fn `SetUpInput`
  (bind _asplayer_controller (cast `PlayerController` (`self.GetController`))
    (:`then`
      (message `EnhancedInputSubsystemInterface.AddMappingContext` (pcsubsystem `EnhancedInputLocalPlayerSubsystem` _asplayer_controller) "/Game/Blueprints/Input/IMC_Input.IMC_Input" 0 (struct)))
    (:`CastFailed`
      (`KismetSystemLibrary.PrintString` "Couldn't find player controller"))))

(fn `UserConstructionScript`)