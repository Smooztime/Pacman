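; Pac-Man game mode that handles level wins, losses and progression through the game instance.
; On BeginPlay it caches the player character and game instance, and counts BP_Bag actors as collectibles left.
; HandleWin, once none remain, reloads ThirdPersonMap, saving score and health and raising enemy speed and level.
; HandleLose reloads the map, resets enemy speed and saves score, or opens MainMenu and resets progress when stored health is depleted.
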(event `self.ReceiveBeginPlay`
  (bind _asbp_base_character (cast `/Game/Pacman/Blueprints/Characters/BP_BaseCharacter` (`GameplayStatics.GetPlayerCharacter` 0)))
  (set `self.Character` _asbp_base_character)
  (bind _outactors (`GameplayStatics.GetAllActorsOfClass` "/Game/Pacman/Blueprints/Collectible/BP_Bag.BP_Bag_C"))
  (set `self.CollectiblesLeft` (`KismetArrayLibrary.Array_Length` _outactors))
  (bind _asgi_base_game_instance (cast `/Game/Pacman/Blueprints/GameInstance/GI_BaseGameInstance` (`GameplayStatics.GetGameInstance`)))
  (set `self.BaseGameInstance` _asgi_base_game_instance))

(fn `HandleLose`
  (`GameplayStatics.OpenLevel` "ThirdPersonMap")
  (set `/Game/Pacman/Blueprints/GameInstance/GI_BaseGameInstance.EnemySpeed` 0.0 (`self.BaseGameInstance`))
  (set `/Game/Pacman/Blueprints/GameInstance/GI_BaseGameInstance.PlayerScore` (`/Game/Pacman/Blueprints/Characters/BP_BaseCharacter.CurrentScore` (`self.Character`)) (`self.BaseGameInstance`))
  (if (<= (`/Game/Pacman/Blueprints/GameInstance/GI_BaseGameInstance.PlayerHealth` (`self.BaseGameInstance`)) 0)
    (`GameplayStatics.OpenLevel` "MainMenu")
    (set `/Game/Pacman/Blueprints/GameInstance/GI_BaseGameInstance.PlayerScore` 0 (`self.BaseGameInstance`))
    (set `/Game/Pacman/Blueprints/GameInstance/GI_BaseGameInstance.PlayerHealth` 3 (`self.BaseGameInstance`))
    (set `/Game/Pacman/Blueprints/GameInstance/GI_BaseGameInstance.CurrentLevel` 1 (`self.BaseGameInstance`))
    (`/Game/Pacman/Blueprints/GameInstance/GI_BaseGameInstance.PlayBGMusics` (`self.BaseGameInstance`) null 0.0 false false)))

(fn `HandleWin`
  (bind _basegameinstance (`self.BaseGameInstance`))
  (bind _basegameinstance_2 (`self.BaseGameInstance`))
  (if (== (`self.CollectiblesLeft`) (`self.Empty`))
    (`GameplayStatics.OpenLevel` "ThirdPersonMap")
    (set `/Game/Pacman/Blueprints/GameInstance/GI_BaseGameInstance.PlayerScore` (`/Game/Pacman/Blueprints/Characters/BP_BaseCharacter.CurrentScore` (`self.Character`)) (`self.BaseGameInstance`))
    (set `/Game/Pacman/Blueprints/GameInstance/GI_BaseGameInstance.PlayerHealth` (`/Game/Pacman/Blueprints/Characters/BP_BaseCharacter.CurrentHealth` (`self.Character`)) _basegameinstance)
    (set `/Game/Pacman/Blueprints/GameInstance/GI_BaseGameInstance.EnemySpeed` (+ (`/Game/Pacman/Blueprints/GameInstance/GI_BaseGameInstance.EnemySpeed` _basegameinstance) (`self.SpeedIncrease`)) _basegameinstance)
    (set `/Game/Pacman/Blueprints/GameInstance/GI_BaseGameInstance.CurrentLevel` (+ (`/Game/Pacman/Blueprints/GameInstance/GI_BaseGameInstance.CurrentLevel` _basegameinstance_2) (`self.LevelIncrease`)) _basegameinstance_2)))

(fn `UserConstructionScript`)