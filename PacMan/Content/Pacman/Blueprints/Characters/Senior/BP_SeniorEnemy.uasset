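; Senior enemy character in the Pacman game that senses the player, attacks in melee and teleports back to its start location on EnemyDestroy.
; AI Perception sight results set the controller's blackboard seen-player key, while heard locations go to it as points of interest.
; AttackPlayer plays a montage when a forward sphere trace hits a BP_BaseCharacter.
; Damage comes from overlaps on a hand-socket collider, disabled at BeginPlay and switchable through ChangeHandCollision.
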(event `self.ReceiveTick`
  (params (DeltaSeconds :type "Float (single-precision)")))

(event `self.ReceiveBeginPlay`
  (set `self.StartLocation` (`SceneComponent.RelativeLocation` (`self.CapsuleComponent`)))
  (bind _asaic_senior_controller (cast `/Game/Pacman/Blueprints/Characters/Senior/AI/AIC_SeniorController` (`self.GetController`)))
  (set `self.EnemyController` _asaic_senior_controller)
  (`self.ChangeHandCollision` "NoCollision")
  (bind _asgi_base_game_instance (cast `/Game/Pacman/Blueprints/GameInstance/GI_BaseGameInstance` (`GameplayStatics.GetGameInstance`)))
  (set `self.EnemySpeedIncrease` (`/Game/Pacman/Blueprints/GameInstance/GI_BaseGameInstance.EnemySpeed` _asgi_base_game_instance)))

(event `self.RightHandCollision.OnComponentBeginOverlap`
  (params (OverlappedComponent :type "PrimitiveComponent Object Reference") (OtherActor :type "Actor Object Reference") (OtherComp :type "PrimitiveComponent Object Reference") (OtherBodyIndex :type Integer) (bFromSweep :type Boolean) (SweepResult :type "HitResult Structure (by ref)"))
  (bind _asbp_base_character (cast `/Game/Pacman/Blueprints/Characters/BP_BaseCharacter` OtherActor))
  (`/Game/Pacman/Blueprints/Characters/BP_BaseCharacter.TakeDamage` _asbp_base_character))

(event `EnemyDestroy`
  (`self.K2_TeleportTo` (`self.StartLocation`)))

(event `self.AIPerception.OnPerceptionUpdated`
  (params (UpdatedActors :type "Array of Actor Object Reference (by ref)"))
  (for _array_element UpdatedActors
    (`|ExecutionSequence`
      (:`then_0`
        (bind _success (`self.CanSense` _array_element))
        (if _success
          (`self.SetHasSeenPlayerKey` true)
          (else
            (`self.SetHasSeenPlayerKey` false))))
      (:`then_1`
        (bind (_success_2 _stimulus) (`self.CanSense` _array_element "NewEnumerator1"))
        (if _success_2
          (`/Game/Pacman/Blueprints/Characters/Senior/AI/AIC_SeniorController.ExplorePointOfInterest` (`self.EnemyController`) (`.StimulusLocation` (break `AIStimulus` _stimulus))))))))

(event `AttackPlayer`
  (bind _returnvalue (`self.K2_GetActorLocation`))
  (bind (_outhit _returnvalue_2) (`KismetSystemLibrary.SphereTraceSingleForObjects` _returnvalue (+ _returnvalue (* (`KismetMathLibrary.GetForwardVector` (`self.K2_GetActorRotation`)) 250.0)) 120.0 (`|MakeArray` "ObjectTypeQuery3" :!type "EObjectTypeQuery Enum")))
  (if _returnvalue_2
    (cast `/Game/Pacman/Blueprints/Characters/BP_BaseCharacter` (`.HitActor` (`GameplayStatics.BreakHitResult` _outhit)))
    (`self.PlayAnimMontage` "/Game/Pacman/Assets/Characters/Enemy/Animation/AM_SeniorAttack.AM_SeniorAttack")))

(fn `CanSense`
  (params (Actor :type "Actor Object Reference") (Sense :type "/Game/Scripts/E_AISense Enum" :default "NewEnumerator0"))
  (returns (Success :type Boolean) (Stimulus :type "AIStimulus Structure"))
  (bind _info (`AIPerceptionComponent.GetActorsPerception` (`self.AIPerception`) Actor))
  (for _array_element (`.LastSensedStimuli` (break `ActorPerceptionBlueprintInfo` _info))
    (bind _returnvalue (`AIPerceptionSystem.GetSenseClassForStimulus` _array_element))
    (if (== _returnvalue (select `/Game/Scripts/E_AISense` Sense :`NewEnumerator0` "/Script/AIModule.AISense_Sight" :`NewEnumerator1` "/Script/AIModule.AISense_Hearing" :!type "Object Class Reference"))
      (return (`.bSuccessfullySensed` (break `AIStimulus` _array_element)) _array_element))))

(fn `ChangeHandCollision`
  (params (Collision :type "ECollisionEnabled Enum" :default "NoCollision"))
  (`PrimitiveComponent.SetCollisionEnabled` (`self.RightHandCollision`) Collision))

(fn `SetHasSeenPlayerKey`
  (params (HasSeenPlayer :type Boolean))
  (`BlackboardComponent.SetValueAsBool` (`AIController.Blackboard` (`self.EnemyController`)) (`self.HasSeenPlayerKey`) HasSeenPlayer))

(fn `UserConstructionScript`
  (`SceneComponent.K2_AttachToComponent` (`self.RightHandCollision`) (`self.Mesh`) "RightHand" "KeepRelative" "KeepRelative" "KeepRelative" true))