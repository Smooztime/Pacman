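; Player character for the Pacman game, with Enhanced Input movement that emits AI noise, a charged dash and a pause menu toggle.
; Holding dash builds launch force while draining stamina; release launches forward, empties stamina and disables further dashes.
; Hitting a BP_SeniorEnemy mid-dash destroys it and decrements the game mode's enemy count.
; Score, health and level load from the game instance; HUD helpers update the display, and TakeDamage triggers HandleLose.
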(event `self.ReceiveBeginPlay`
  (set `self.bCanDash` true)
  (bind _output_get (set `self.CurrentSP` (`self.MaxSP`)))
  (`self.Set UIStamina` _output_get)
  (bind _asgi_base_game_instance (cast `/Game/Pacman/Blueprints/GameInstance/GI_BaseGameInstance` (`GameplayStatics.GetGameInstance`)))
  (set `self.BaseGameInstance` _asgi_base_game_instance)
  (`self.UpdateCurrentScore` (`/Game/Pacman/Blueprints/GameInstance/GI_BaseGameInstance.PlayerScore` _asgi_base_game_instance))
  (set `self.CurrentHealth` (`/Game/Pacman/Blueprints/GameInstance/GI_BaseGameInstance.PlayerHealth` _asgi_base_game_instance))
  (`self.UpdateCurrentLevel` (`/Game/Pacman/Blueprints/GameInstance/GI_BaseGameInstance.CurrentLevel` _asgi_base_game_instance))
  (`self.UpdateHighScore` (`/Game/Pacman/Blueprints/GameInstance/GI_BaseGameInstance.PlayerHighScore` _asgi_base_game_instance)))

(event `self.ReceivePossessed`
  (params (NewController :type "Controller Object Reference"))
  (`self.SetUpInput`))

(event `EnhancedInput|/Game/Pacman/Blueprints/Input/IA_Movement`
  (params (ActionValue :type "Vector2D Structure") (ElapsedSeconds :type "Float (double-precision)") (TriggeredSeconds :type "Float (double-precision)") (InputAction :type "InputAction Object Reference" :default "/Game/Pacman/Blueprints/Input/IA_Movement.IA_Movement"))
  (:`Triggered`
    (if (`self.CanMove`)
      (`self.Movement` ActionValue)
      (`self.MakeNoise` 1.0 self (`self.K2_GetActorLocation`))
      (if (>= (`KismetMathLibrary.VSizeXY` (`MovementComponent.Velocity` (`self.CharacterMovement`))) 300.0)
        (set `self.bIsMove` true))))
  (:`Completed`
    (set `self.bIsMove` false)))

(event `EnhancedInput|/Game/Pacman/Blueprints/Input/IA_ChargeDash`
  (params (ActionValue :type Boolean) (ElapsedSeconds :type "Float (double-precision)") (TriggeredSeconds :type "Float (double-precision)") (InputAction :type "InputAction Object Reference" :default "/Game/Pacman/Blueprints/Input/IA_ChargeDash.IA_ChargeDash"))
  (:`Triggered`
    (if (`self.bCanDash`)
      (set `self.CurrentState` "NewEnumerator4")
      (`self.SetForce`)))
  (:`Completed`
    (if (`|EnumEquality` (`self.CurrentState`) "NewEnumerator4")
      (`GameplayStatics.PlaySound2D` "/Game/Pacman/Assets/Sounds/SFX/Dash.Dash" 1.0 1.0 0.0 null null)
      (`self.Dash`)
      (set `self.CurrentForce` 0.0)
      (bind _output_get (set `self.CurrentSP` 0.0))
      (`self.Set UIStamina` _output_get)
      (set `self.bCanDash` false)
      (`KismetSystemLibrary.Delay` 0.15)
      (set `self.CurrentState` "NewEnumerator0"))))

(event `EnhancedInput|/Game/Pacman/Blueprints/Input/IA_ESC`
  (params (ActionValue :type Boolean) (ElapsedSeconds :type "Float (double-precision)") (TriggeredSeconds :type "Float (double-precision)") (InputAction :type "InputAction Object Reference" :default "/Game/Pacman/Blueprints/Input/IA_ESC.IA_ESC"))
  (bind _returnvalue (`GameplayStatics.GetPlayerController` 0))
  (bind _returnvalue_2 (`GameplayStatics.GetPlayerController` 0))
  (:`Started`
    (if (not (`self.bIsPauseMenuOpen`))
      (set `self.bIsPauseMenuOpen` true)
      (bind _returnvalue_3 (`|CreateWidget` "/Game/Pacman/Blueprints/HUD/WB_PauseMenu.WB_PauseMenu_C"))
      (bind _output_get (set `self.PauseMenuUI` _returnvalue_3))
      (`UserWidget.AddToViewport` _output_get 0)
      (`WidgetBlueprintLibrary.SetInputMode_GameAndUIEx` _returnvalue_2 (`self.PauseMenuUI`))
      (set `PlayerController.bShowMouseCursor` true _returnvalue_2)
      (`GameplayStatics.SetGamePaused` true)
      (else
        (set `self.bIsPauseMenuOpen` false)
        (`Widget.RemoveFromParent` (`self.PauseMenuUI`))
        (`GameplayStatics.SetGamePaused` false)
        (`WidgetBlueprintLibrary.SetInputMode_GameOnly` _returnvalue)
        (set `PlayerController.bShowMouseCursor` false _returnvalue)))))

(event `self.CapsuleComponent.OnComponentHit`
  (params (HitComponent :type "PrimitiveComponent Object Reference") (OtherActor :type "Actor Object Reference") (OtherComp :type "PrimitiveComponent Object Reference") (NormalImpulse :type "Vector Structure") (Hit :type "HitResult Structure (by ref)"))
  (bind _asbp_senior_enemy (cast `/Game/Pacman/Blueprints/Characters/Senior/BP_SeniorEnemy` OtherActor))
  (if (`|EnumEquality` (`self.CurrentState`) "NewEnumerator2")
    (`/Game/Pacman/Blueprints/Characters/Senior/BP_SeniorEnemy.EnemyDestroy` _asbp_senior_enemy)
    (bind _asbp_base_game_mode (cast `/Game/Pacman/Blueprints/GameMode/BP_BaseGameMode` (`GameplayStatics.GetGameMode`)))
    (bind _result (`/Engine/EditorBlueprintResources/StandardMacros.DecrementInt` (`/Game/Pacman/Blueprints/GameMode/BP_BaseGameMode.EnemiesLeft` _asbp_base_game_mode))
      (:`  `
        (set `/Game/Pacman/Blueprints/GameMode/BP_BaseGameMode.EnemiesLeft` _result _asbp_base_game_mode)))))

(fn `AddForceToDash`)

(fn `CanMove`
  (returns (CanMove :type Boolean))
  (return (`|EnumEquality` (`self.CurrentState`) "NewEnumerator0")))

(fn `Dash`
  (set `self.CurrentState` "NewEnumerator2")
  (`self.LaunchCharacter` (* (`SceneComponent.GetForwardVector` (`self.CapsuleComponent`)) (`self.CurrentForce`))))

(fn `Movement`
  (params (AxisValue :type "Vector2D Structure"))
  (`self.AddMovementInput` (`KismetMathLibrary.Vector_Right`) AxisValue_X)
  (`self.AddMovementInput` (`KismetMathLibrary.Vector_Forward`) AxisValue_Y))

(fn `ReduceSP`
  (bind _output_get (set `self.CurrentSP` (`KismetMathLibrary.FClamp` (- (`self.CurrentSP`) (/ (`self.ForcePerSecond`) (`self.MaxSP`))) 0.0 (`self.MaxSP`))))
  (`self.PlayerHUD`
    (:`then`
      _)
    (:`else`
      (`self.SetupHUD`)))
  (`/Game/Pacman/Blueprints/HUD/BP_PlayerHUD.UpdateStaminaUI` (`self.PlayerHUD`) 0.0 (`self.SetStaminaPercent` _output_get)))

(fn `Set UIStamina`
  (params (CurrentSP :type "Float (double-precision)"))
  (bind _output_get (set `self.CurrentSP` CurrentSP))
  (`self.PlayerHUD`
    (:`then`
      _)
    (:`else`
      (`self.SetupHUD`)))
  (`/Game/Pacman/Blueprints/HUD/BP_PlayerHUD.UpdateStaminaUI` (`self.PlayerHUD`) 0.0 (`self.SetStaminaPercent` _output_get)))

(fn `SetForce`
  (set `self.CurrentForce` (`KismetMathLibrary.FClamp` (+ (`self.CurrentForce`) (`self.ForcePerSecond`)) 0.0 (`self.MaxForce`)))
  (`self.ReduceSP`))

(fn `SetStaminaPercent`
  (params (CurrentSP :type "Float (double-precision)"))
  (returns (StaminaPercent :type "Float (double-precision)"))
  (return (/ CurrentSP (`self.MaxSP`))))

(fn `SetupHUD`
  (bind _asplayer_controller (cast `PlayerController` (`self.GetController`)))
  (bind _asbp_player_hud (cast `/Game/Pacman/Blueprints/HUD/BP_PlayerHUD` (`PlayerController.GetHUD` _asplayer_controller)))
  (bind _output_get (set `self.PlayerHUD` _asbp_player_hud))
  (`/Game/Pacman/Blueprints/HUD/BP_PlayerHUD.UpdateScoreUI` _output_get (`self.CurrentScore`)))

(fn `SetUpInput`
  (bind _asplayer_controller (cast `PlayerController` (`self.GetController`))
    (:`then`
      (message `EnhancedInputSubsystemInterface.AddMappingContext` (pcsubsystem `EnhancedInputLocalPlayerSubsystem` _asplayer_controller) "/Game/Pacman/Blueprints/Input/IMC_Input.IMC_Input" 0 (struct)))
    (:`CastFailed`
      (`KismetSystemLibrary.PrintString` "Couldn't find player controller"))))

(fn `TakeDamage`
  (bind _result (`/Engine/EditorBlueprintResources/StandardMacros.DecrementInt` (`self.CurrentHealth`))
    (:`  `
      (set `self.CurrentHealth` _result)
      (set `/Game/Pacman/Blueprints/GameInstance/GI_BaseGameInstance.PlayerHealth` (`self.CurrentHealth`) (`self.BaseGameInstance`))
      (bind _asbp_base_game_mode (cast `/Game/Pacman/Blueprints/GameMode/BP_BaseGameMode` (`GameplayStatics.GetGameMode`)))
      (`/Game/Pacman/Blueprints/GameMode/BP_BaseGameMode.HandleLose` _asbp_base_game_mode))))

(fn `UpdateCollectibles`
  (params (Collectible :type Integer))
  (`self.PlayerHUD`
    (:`then`
      _)
    (:`else`
      (`self.SetupHUD`)))
  (`/Game/Pacman/Blueprints/HUD/BP_PlayerHUD.UpdateCollectiblesUI` (`self.PlayerHUD`) Collectible))

(fn `UpdateCurrentLevel`
  (params (CurrentLevel :type Integer))
  (bind _output_get (set `self.CurrentLevel` CurrentLevel))
  (`self.PlayerHUD`
    (:`then`
      _)
    (:`else`
      (`self.SetupHUD`)))
  (`/Game/Pacman/Blueprints/HUD/BP_PlayerHUD.UpdateLevelUI` (`self.PlayerHUD`) _output_get))

(fn `UpdateCurrentScore`
  (params (CurrentScore :type Integer))
  (bind _output_get (set `self.CurrentScore` CurrentScore))
  (`self.PlayerHUD`
    (:`then`
      _)
    (:`else`
      (`self.SetupHUD`)))
  (`/Game/Pacman/Blueprints/HUD/BP_PlayerHUD.UpdateScoreUI` (`self.PlayerHUD`) _output_get))

(fn `UpdateHighScore`
  (params (HighScore :type Integer))
  (bind _output_get (set `self.HighScore` HighScore))
  (`self.PlayerHUD`
    (:`then`
      _)
    (:`else`
      (`self.SetupHUD`)))
  (`/Game/Pacman/Blueprints/HUD/BP_PlayerHUD.UpdateHighScoreUI` (`self.PlayerHUD`) _output_get))

(fn `UserConstructionScript`)