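; BP_Collectible is a Pacman pickup that animates in place and is destroyed when a BP_BaseCharacter touches it.
; The BagMove timeline lerps the mesh between StartPoint and Destination from BeginPlay, while Tick spins the actor at a frame-rate-independent yaw rate.
; Box overlap stores the character as Player, then calls TakeItem, which destroys the actor.
; A SubtractAmount helper decrements a passed-in count, but nothing here calls it.
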(event `self.ReceiveBeginPlay`
  (bind (_direction _alpha) (`Timeline|BagMove`)
    (:`Update`
      (`SceneComponent.K2_SetRelativeLocation` (`self.CollectibleMesh`) (`KismetMathLibrary.VLerp` (`self.StartPoint`) (`self.Destination`) _alpha) false false))))

(event `self.ReceiveTick`
  (params (DeltaSeconds :type "Float (single-precision)"))
  (`self.K2_AddActorLocalRotation` (`KismetMathLibrary.MakeRotator` 0.0 0.0 (* DeltaSeconds (`self.CollectibleRotation`)))))

(event `self.Box.OnComponentBeginOverlap`
  (params (OverlappedComponent :type "PrimitiveComponent Object Reference") (OtherActor :type "Actor Object Reference") (OtherComp :type "PrimitiveComponent Object Reference") (OtherBodyIndex :type Integer) (bFromSweep :type Boolean) (SweepResult :type "HitResult Structure (by ref)"))
  (bind _asbp_base_character (cast `/Game/Pacman/Blueprints/Characters/BP_BaseCharacter` OtherActor))
  (set `self.Player` _asbp_base_character)
  (`self.TakeItem`))

(event `TakeItem`
  (`self.K2_DestroyActor`))

(fn `SubtractAmount`
  (params (CollectiblesAmount :type Integer))
  (returns (SubtractAmount :type Integer))
  (bind _result (`/Engine/EditorBlueprintResources/StandardMacros.DecrementInt` CollectiblesAmount)
    (:`  `
      (return _result))))

(fn `UserConstructionScript`)