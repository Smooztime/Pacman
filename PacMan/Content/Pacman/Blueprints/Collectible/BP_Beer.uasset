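; BP_Beer is a Pacman collectible that refills the player's stamina and enables dashing when taken.
; TakeItem sets CanDash, restores CurrentSP to MaxSP, updates the stamina UI, then runs the parent pickup logic.
; SetPercentToUI runs the player's HUD setup if the HUD is invalid, then sends it the SP value divided by ToPercent.
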(event `self.TakeItem`
  (bind _player (`self.Player`))
  (set `/Game/Pacman/Blueprints/Characters/BP_BaseCharacter.bCanDash` true (`self.Player`))
  (bind _output_get (set `/Game/Pacman/Blueprints/Characters/BP_BaseCharacter.CurrentSP` (`/Game/Pacman/Blueprints/Characters/BP_BaseCharacter.MaxSP` _player) _player))
  (`self.SetPercentToUI` _output_get)
  (`parent.TakeItem`))

(fn `SetPercentToUI`
  (params (A :type "Float (double-precision)"))
  (bind _playerhud (`/Game/Pacman/Blueprints/Characters/BP_BaseCharacter.PlayerHUD` (`self.Player`))
    (:`then`
      _)
    (:`else`
      (`/Game/Pacman/Blueprints/Characters/BP_BaseCharacter.SetupHUD` (`self.Player`))))
  (`/Game/Pacman/Blueprints/HUD/BP_PlayerHUD.UpdateStaminaUI` _playerhud 0.0 (/ A (`self.ToPercent`))))

(fn `UserConstructionScript`
  (`parent.UserConstructionScript`))