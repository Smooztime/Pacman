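; Animation notify for enemy attacks that picks a hit or miss sound, without applying damage.
; On firing, it sphere-traces a short distance ahead of the mesh owner for Pawns, ignoring all BP_SeniorEnemy actors.
; If the hit actor is the first BP_BaseCharacter found, it plays Slap through GI_BaseGameInstance, persisting across level transitions.
; Otherwise it plays a 2D Swoosh.
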(fn `Received_Notify`
  (params (MeshComp :type "SkeletalMeshComponent Object Reference") (Animation :type "AnimSequenceBase Object Reference") (EventReference :type "AnimNotifyEventReference Structure (by ref)"))
  (returns (ReturnValue :type Boolean))
  (bind _returnvalue (`Actor.K2_GetActorLocation` (`ActorComponent.GetOwner` MeshComp)))
  (bind _outactors (`GameplayStatics.GetAllActorsOfClass` "/Game/Pacman/Blueprints/Characters/Senior/BP_SeniorEnemy.BP_SeniorEnemy_C"))
  (bind _outhit (`KismetSystemLibrary.SphereTraceSingleForObjects` _returnvalue (+ _returnvalue (* (`Actor.GetActorForwardVector` (`ActorComponent.GetOwner` MeshComp)) 90.0)) 50.0 (`|MakeArray` "ObjectTypeQuery3" :!type "EObjectTypeQuery Enum") false _outactors))
  (bind _outactors_2 (`GameplayStatics.GetAllActorsOfClass` "/Game/Pacman/Blueprints/Characters/BP_BaseCharacter.BP_BaseCharacter_C"))
  (if (== (`.HitActor` (`GameplayStatics.BreakHitResult` _outhit)) (`|GetArrayItem` _outactors_2))
    (bind _asgi_base_game_instance (cast `/Game/Pacman/Blueprints/GameInstance/GI_BaseGameInstance` (`GameplayStatics.GetGameInstance`)))
    (`/Game/Pacman/Blueprints/GameInstance/GI_BaseGameInstance.PlayBGSFX` _asgi_base_game_instance "/Game/Pacman/Assets/Sounds/SFX/Slap.Slap" 1.0 true)
    (else
      (`GameplayStatics.PlaySound2D` "/Game/Pacman/Assets/Sounds/SFX/Swoosh.Swoosh" 1.0 1.0 0.0 null null)))
  (return false))